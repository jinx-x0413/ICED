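; Player pawn for selecting glTF asset actors with the mouse and driving runtime translate, rotate and scale gizmos through TransformerPawn.
; BeginPlay retries until TransformerPawn is valid, then assigns gizmo classes and binds press/release events that set its activation flag.
; Left click traces for gizmos and selects any GltfAssetActor under the cursor, while release clears the gizmo domain.
; Key 1 cycles transformation modes, and Tick updates transforms while the gizmo state is active.
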(event `self.ReceiveBeginPlay`
  ;[0 0 0] Initialize Gizmo
  (bind _transformerpawn (`self.TransformerPawn` :!label _label)
    (:`then`
      (set `TransformerPawn.TranslationGizmoClass` "/RuntimeTransformer/GizmoExamples/BP_TranslationGizmo_Example.BP_TranslationGizmo_Example_C" _transformerpawn)
      (set `TransformerPawn.RotationGizmoClass` "/RuntimeTransformer/GizmoExamples/BP_Rotation_Gizmo_Example.BP_Rotation_Gizmo_Example_C" _transformerpawn)
      (set `TransformerPawn.ScaleGizmoClass` "/RuntimeTransformer/GizmoExamples/BP_Scale_Gizmo_Example.BP_Scale_Gizmo_Example_C" _transformerpawn)
      (add `TransformerPawn.OnGizmoPressed` (`self.TransformerPawn`) (delegate `CustomEvent_2`))
      (add `TransformerPawn.OnGizmoReleased` (`self.TransformerPawn`) (delegate `CustomEvent_3`)))
    (:`else`
      (`KismetSystemLibrary.Delay` 0.2)
      (goto _label))))

(event `Key|LeftMouseButton`
  (params (Key :type "Key Structure"))
  (bind (_hitresult _returnvalue) (`PlayerController.GetHitResultUnderCursorByChannel` (`GameplayStatics.GetPlayerController` 0) "TraceTypeQuery2" true))
  (bind (_asgltf_asset_actor _bsuccess) (cast `GltfAssetActor` (`.HitActor` (`GameplayStatics.BreakHitResult` _hitresult)) :!pure true))
  ;[0 0 0] Control Actor
  (:`Pressed`
    (`|ExecutionSequence`
      (:`then_0`
        (`TransformerPawn.MouseTraceByObjectTypes` (`self.TransformerPawn`) 5000000.0 (`|MakeArray` "ECC_WorldStatic" "ECC_WorldDynamic" :!type "ECollisionChannel Enum") (`self.IgnoreItem`) false))
      (:`then_1`
        (if (and _bsuccess _returnvalue)
          (`self.SelectActor` _asgltf_asset_actor)))))
  (:`Released`
    (`TransformerPawn.ClearDomain` (`self.TransformerPawn`))))

(event `CustomEvent_2`
  (params (InTransform :type "Transform Structure"))
  ;[0 0 0] Initialize Gizmo
  (set `TransformerPawn.bIsActivatingGizmo` true (`self.TransformerPawn`)))

(event `CustomEvent_3`
  (params (InTransform :type "Transform Structure"))
  ;[0 0 0] Initialize Gizmo
  (set `TransformerPawn.bIsActivatingGizmo` false (`self.TransformerPawn`)))

(event `Key|One`
  (params (Key :type "Key Structure"))
  ;[0 0 0] Switch Gizmo
  ; TODO : UI
  (:`Pressed`
    (switch `ETransformationType` (`self.Transformation Type`)
      (:`TT_NoTransform`
        (bind _output_get (set `self.Transformation Type` "TT_Translation" :!label _label_2)))
      (:`TT_Translation`
        (set `self.Transformation Type` "TT_Rotation"))
      (:`TT_Rotation`
        (set `self.Transformation Type` "TT_Scale"))
      (:`TT_Scale`
        (goto _label_2)))
    (`TransformerPawn.SetTransformationType` (`self.TransformerPawn`) _output_get)))

(event `self.ReceiveTick`
  (params (DeltaSeconds :type "Float (single-precision)"))
  (bind _transformerpawn (`self.TransformerPawn`))
  ;[0 0 0] Update Actor
  (if (`TransformerPawn.GetGizmoState` _transformerpawn)
    (`TransformerPawn.UpdateGizmoTransformations` _transformerpawn)))

(fn `UserConstructionScript`)
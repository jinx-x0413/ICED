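; Pawn that lets the player select glTF asset actors at runtime and transform them with move, rotate and scale gizmos.
; BeginPlay waits for a valid TransformerPawn, assigns its example gizmo classes and enables a visible cursor with Game and UI input.
; Left click traces for objects, selects any glTF actor under the cursor and shows the gizmo, with release clearing the domain.
; The 1 key cycles the transformation type.
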(event `self.ReceiveBeginPlay`
  (bind _transformerpawn (`self.TransformerPawn`))
  (`self.TransformerPawn` :!label _label
    (:`then`
      (`|ExecutionSequence`
        (:`then_0`
          (set `TransformerPawn.TranslationGizmoClass` "/RuntimeTransformer/GizmoExamples/BP_TranslationGizmo_Example.BP_TranslationGizmo_Example_C" _transformerpawn)
          (`TransformerPawn.ForceCreateGizmo` _transformerpawn)
          (bind _asplayer_controller (cast `PlayerController` (`self.GetController`)))
          (`WidgetBlueprintLibrary.SetInputMode_GameAndUIEx` _asplayer_controller null)
          (set `PlayerController.bShowMouseCursor` true _asplayer_controller))
        (:`then_1`
          (set `TransformerPawn.RotationGizmoClass` "/RuntimeTransformer/GizmoExamples/BP_Rotation_Gizmo_Example.BP_Rotation_Gizmo_Example_C" _transformerpawn))
        (:`then_2`
          (set `TransformerPawn.ScaleGizmoClass` "/RuntimeTransformer/GizmoExamples/BP_Scale_Gizmo_Example.BP_Scale_Gizmo_Example_C" _transformerpawn))))
    (:`else`
      (`KismetSystemLibrary.Delay` 0.2)
      (goto _label))))

(event `Key|LeftMouseButton`
  (params (Key :type "Key Structure"))
  (:`Pressed`
    (`|ExecutionSequence`
      (:`then_0`
        (`TransformerPawn.MouseTraceByObjectTypes` (`self.TransformerPawn`) 500000000.0 (`|MakeArray` "ECC_WorldStatic" "ECC_WorldDynamic" :!type "ECollisionChannel Enum") (`|MakeArray` null :!type "Actor Object Reference") false))
      (:`then_1`
        (bind _asgltf_asset_actor (cast `GltfAssetActor` (`.HitActor` (`GameplayStatics.BreakHitResult` (`PlayerController.GetHitResultUnderCursorByChannel` (`GameplayStatics.GetPlayerController` 0) "TraceTypeQuery1" true)))))
        (`TransformerPawn.SetCurrentSelectActor` (`self.TransformerPawn`) _asgltf_asset_actor)
        (`self.ShowGizmo`))))
  (:`Released`
    (`TransformerPawn.ClearDomain` (`self.TransformerPawn`))))

(event `Key|One`
  (params (Key :type "Key Structure"))
  (:`Pressed`
    (switch `ETransformationType` (`self.Transformation Type`)
      (:`TT_NoTransform`
        (bind _output_get (set `self.Transformation Type` "TT_Translation" :!label _label_2)))
      (:`TT_Translation`
        (set `self.Transformation Type` "TT_Rotation"))
      (:`TT_Rotation`
        (set `self.Transformation Type` "TT_Scale"))
      (:`TT_Scale`
        (goto _label_2)))
    (`TransformerPawn.SetTransformationType` (`self.TransformerPawn`) _output_get)))

(fn `UserConstructionScript`)
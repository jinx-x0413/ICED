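; BP_PC shows the main UI and loads glTF models at runtime for assembly and disassembly content.
; On BeginPlay it adds WBP_Main, builds a placeholder model from a hardcoded filename and binds the HTTP request object's DestroyGltfAssetActor event.
; That event loads the cart's file from the project's Resource folder.
; Each load spawns a scaled asset actor and constructs both content sets using WBP_ComponentItem scene-capture widgets.
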(event `self.ReceiveBeginPlay`
  (`|ExecutionSequence`
    (:`then_0`
      ;[1 1 1] Http :: Login
      (bind _returnvalue (`|CreateWidget` "/Game/WBP_Main.WBP_Main_C"))
      (`UserWidget.AddToViewport` _returnvalue 0))
    (:`then_1`
      ;[1 1 1] Construct Content
      ; TODO : Change FileName w/ HttpRequest
      (`self.ConstructContent` "dsdds.glb"))
    (:`then_2`
      ;[0 0 0] Bind Cart Onclick
      (bind _returnvalue_2 (`EntryPoint.GetHttpRequest`))
      (add `HttpRequest.DestroyGltfAssetActor` _returnvalue_2 (delegate `DestroyGltfAssetActor_Event`)))))

(event `ConstructContent`
  (params (InFileName :type String))
  ;[0 0 0] CosntructContent
  ;;[0 0 0] Build AssetActor
  (bind _returnvalue (`glTFRuntimeFunctionLibrary.glTFLoadAssetFromFilename` (`KismetStringLibrary.Concat_StrStr` (`KismetSystemLibrary.GetProjectDirectory`) "Resource/" InFileName) false (make `glTFRuntimeConfig` "Default")))
  (bind _returnvalue_2 (`EntryPoint.CreateGltfAssetActor` "/Script/AssetActor.GltfAssetActor" (`KismetMathLibrary.MakeTransform` (150.0 0.0 200.0) (struct) (5.0 5.0 5.0)) _returnvalue))
  (set `self.____GltfAssetActor` _returnvalue_2)
  ;;[0 0 0] Build Content
  (`EntryPoint.ConstructAssetContent` _returnvalue_2 "Assembly" "/Game/Widgets/AssetContent/Player/List/WBP_ComponentItem.WBP_ComponentItem_C")
  (`EntryPoint.ConstructAssetContent` _returnvalue_2 "Disassembly" "/Game/Widgets/AssetContent/Player/List/WBP_ComponentItem.WBP_ComponentItem_C"))

(event `DestroyGltfAssetActor_Event`
  ;[0 0 0] Bind Cart Onclick
  (bind _returnvalue (`EntryPoint.GetHttpRequest`))
  (`self.ConstructContent` (`.fileName` (break `Cart` (`HttpRequest.Cart` _returnvalue)))))

(fn `UserConstructionScript`)